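; ShoppingGameInstance is the game instance that handles level unlock progression from earned stars.
; CheckForLevelUnlock unlocks Level 2 once Level 1 has at least one star, then Level 3 on a later check once Level 2 has one.
; Each new unlock sets its flag immediately, then shows the W_LevelUnlocked widget after a short delay.
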(event Custom|CheckForLevelUnlock
  (if (Variables|Default|GetisLevel2Unlocked?)
    (if (not (Variables|Default|GetisLevel3Unlocked?))
      (if (>= (Variables|Default|GetLevel2Stars) 1)
        (Variables|Default|SetisLevel3Unlocked? true)
        (Utilities|FlowControl|Delay 2.0)
        (bind _returnvalue (UserInterface|CreateWidget "/Game/Blueprints/UI/w_LevelUnlocked.w_LevelUnlocked_C"))
        (UserInterface|Viewport|AddtoViewport _returnvalue 0)))
    (elif (>= (Variables|Default|GetLevel1Stars) 1)
      (Variables|Default|SetisLevel2Unlocked? true)
      (Utilities|FlowControl|Delay 2.0)
      (bind _returnvalue_2 (UserInterface|CreateWidget "/Game/Blueprints/UI/w_LevelUnlocked.w_LevelUnlocked_C"))
      (UserInterface|Viewport|AddtoViewport _returnvalue_2 0))))