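; Level manager for Shop Till Ya Drop that starts a round and spawns objective items, hazards and pickups.
; After a short delay on BeginPlay it sends star targets to the game mode and sets up AI on every BP_Spline.
; Objective pickups trigger the next item spawn, while looping timers run alongside for recurring spawns.
; Each spawner shuffles its spawn points, favouring a different map area from last time, with a resettable DoOnce guard.
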(event Custom|GetCurrentLocation
  (params (CurrentItemLocation :type Vector))
  (Variables|Default|SetCurrentItemLocation CurrentItemLocation))

(event Custom|StartGame
  (EventDispatchers|BindEventtoCheckforObjectiveItemPickUp (delegate Custom|SpawnItem))
  (CallFunction|SpawnItem)
  (Utilities|Time|SetTimerbyEvent (EventDispatchers|CreateEvent :!event Custom|Spawn%20Hazard) 5.0 true)
  (Default|SetNameofLevel (.AsShop%20Till%20Ya%20Drop%20Gamemode (Utilities|Casting|CastToShopTillYaDropGamemode (Game|GetGameMode))) (Variables|Default|GetShopTitle))
  (Utilities|Time|SetTimerbyEvent (EventDispatchers|CreateEvent :!event Custom|SpawnPickUps) 6.0 true))

(event Custom|SpawnPickUps
  (bind _itemspawnareas (Variables|Default|GetItemSpawnAreas))
  (Utilities|FlowControl|DoOnce false :!label _label
    (:Completed
      (Utilities|Array|Shuffle _itemspawnareas)
      (bind _array_element (Utilities|Array|ForEachLoopwithBreak _itemspawnareas :!label _label_2)
        (:LoopBody
          (Utilities|IsValid _array_element
            (:Is%20Valid
              (if (not (Utilities|Enum|Equal(Enum) (Variables|/Game/Blueprints/GameControl/Spawn/ObjectiveItemSpawner.ObjectiveItemSpawner_C|GetMapArea _array_element) (Variables|Default|GetPreviousPickUpSpawnArea)))
                (goto _label_2 Break)))))
        (:Completed
          (Utilities|IsValid _array_element
            (:Is%20Valid
              (bind _output_get (Variables|Default|SetItemSpawn _array_element))
              (Variables|Default|SetPreviousPickUpSpawnArea (Variables|/Game/Blueprints/GameControl/Spawn/ObjectiveItemSpawner.ObjectiveItemSpawner_C|GetMapArea _output_get))
              (Default|SpawnPickUp _array_element)
              (goto _label Reset))))))))

(event Custom|Spawn%20Hazard
  (bind _hazardspawnareas (Variables|Default|GetHazardSpawnAreas))
  (Utilities|FlowControl|DoOnce false :!label _label
    (:Completed
      (Utilities|Array|Shuffle _hazardspawnareas)
      (bind _array_element (Utilities|Array|ForEachLoopwithBreak _hazardspawnareas :!label _label_2)
        (:LoopBody
          (Utilities|IsValid _array_element
            (:Is%20Valid
              (if (not (Utilities|Enum|Equal(Enum) (Variables|/Game/Blueprints/GameControl/Spawn/HazardSpawner.HazardSpawner_C|GetMapArea _array_element) (Variables|Default|GetPreviousHazardSpawnArea)))
                (goto _label_2 Break)))))
        (:Completed
          (Utilities|IsValid _array_element
            (:Is%20Valid
              (bind _output_get (Variables|Default|SetHazardSpawn _array_element))
              (Variables|Default|SetPreviousHazardSpawnArea (Variables|/Game/Blueprints/GameControl/Spawn/HazardSpawner.HazardSpawner_C|GetMapArea _output_get))
              (Default|SpawnHazard _output_get)
              (goto _label Reset))))))))

(event Custom|SpawnItem
  (bind _itemspawnareas (Variables|Default|GetItemSpawnAreas))
  (Utilities|FlowControl|DoOnce false :!label _label
    (:Completed
      (Utilities|Array|Shuffle _itemspawnareas)
      (bind _array_element (Utilities|Array|ForEachLoopwithBreak _itemspawnareas :!label _label_2)
        (:LoopBody
          (Utilities|IsValid _array_element
            (:Is%20Valid
              (if (not (Utilities|Enum|Equal(Enum) (Variables|/Game/Blueprints/GameControl/Spawn/ObjectiveItemSpawner.ObjectiveItemSpawner_C|GetMapArea _array_element) (Variables|Default|GetCurrentArea)))
                (goto _label_2 Break)))))
        (:Completed
          (Utilities|IsValid _array_element
            (:Is%20Valid
              (bind _output_get (Variables|Default|SetItemSpawn _array_element))
              (Variables|Default|SetCurrentArea (Variables|/Game/Blueprints/GameControl/Spawn/ObjectiveItemSpawner.ObjectiveItemSpawner_C|GetMapArea _output_get))
              (Default|SpawnItem _output_get)
              (goto _label Reset))))))))

(event EventBeginPlay
  (Utilities|FlowControl|Delay 0.1)
  (bind _asshop_till_ya_drop_pawn (Utilities|Casting|CastToShopTillYaDropPawn (Game|GetPlayerCharacter 0)))
  (Variables|Default|SetPlayer _asshop_till_ya_drop_pawn)
  (Default|SetTargetScores (.AsShop%20Till%20Ya%20Drop%20Gamemode (Utilities|Casting|CastToShopTillYaDropGamemode (Game|GetGameMode))) (Variables|Default|GetStarAmounts))
  (bind _outactors (Actor|GetAllActorsOfClass "/Game/Blueprints/AI/BP_Spline.BP_Spline_C"))
  (for _array_element _outactors
    (Default|SetUpAI _array_element))
  (CallFunction|StartGame))

(fn ConstructionScript)