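; Game mode for Shop Till Ya Drop, a timed shopping game that ends when the player character drops.
; Setup prepares the character and shows a countdown widget; Pre-Game removes it, enables input and starts play.
; A looping one-second timer drains TimeTillDrop, then triggers ragdoll death and Post-Game.
; Post-Game copies weight and item totals and animates end-screen stars; CalculateScore, which weights bought items double, is not called here.
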(event Custom|Init
  (bind _asshop_till_ya_drop_pawn (Utilities|Casting|CastToShopTillYaDropPawn (Game|GetPlayerCharacter 0)))
  (Variables|Default|SetPlayerCharacter _asshop_till_ya_drop_pawn))

(event Custom|Timer
  (bind _playercharacter (Variables|Default|GetPlayerCharacter))
  (Utilities|IsValid _playercharacter
    (:Is%20Valid
      (bind _output_get (Variables|/Game/Blueprints/Character/ShopTillYaDropPawn.ShopTillYaDropPawn_C|SetTimeTillDrop _playercharacter (- (Variables|/Game/Blueprints/Character/ShopTillYaDropPawn.ShopTillYaDropPawn_C|GetTimeTillDrop _playercharacter) 1.0)))
      (if (<= _output_get 0.0)
        (Default|RagdollDeath (Variables|Default|GetPlayerCharacter))
        (Utilities|Time|ClearandInvalidateTimerbyHandle (Variables|Default|GetTimerControl))
        (CallFunction|Post-Game)))))

(event Custom|Set-Up
  (Default|SetUpCharacter (Variables|Default|GetPlayerCharacter))
  (bind _returnvalue (UserInterface|CreateWidget "/Game/Blueprints/UI/w_Countdown.w_Countdown_C"))
  (bind _output_get (Variables|Default|SetStartCountdown _returnvalue))
  (UserInterface|Viewport|AddtoViewport _output_get 0))

(event Custom|SetNameOfLevel
  (params (ShopName :type ShopNames%20Enum :default "NewEnumerator0"))
  (Variables|Default|SetShopName ShopName))

(event Custom|Pre-Game
  (Widget|RemovefromParent (Variables|Default|GetStartCountdown))
  (Default|AllowInput (Variables|Default|GetPlayerCharacter))
  (CallFunction|In-Game))

(event Custom|In-Game
  (bind _returnvalue (Utilities|Time|SetTimerbyEvent (delegate Custom|Timer) 1.0 true))
  (Variables|Default|SetTimerControl _returnvalue))

(event Custom|Post-Game
  (bind _playercharacter (Variables|Default|GetPlayerCharacter))
  (Variables|Default|SetTotalWeight (Variables|/Game/Blueprints/Character/ShopTillYaDropPawn.ShopTillYaDropPawn_C|GetTotalWeight _playercharacter))
  (Variables|Default|SetItemsCarried (Variables|/Game/Blueprints/Character/ShopTillYaDropPawn.ShopTillYaDropPawn_C|GetItemsPickedUp _playercharacter))
  (Variables|Default|SetItemsBought (Variables|/Game/Blueprints/Character/ShopTillYaDropPawn.ShopTillYaDropPawn_C|GetItemsDroppedOff _playercharacter))
  (bind _returnvalue (UserInterface|CreateWidget "/Game/Blueprints/UI/w_EndScreen.w_EndScreen_C"))
  (UserInterface|Viewport|AddtoViewport _returnvalue 0)
  (Default|StarAnim _returnvalue (Variables|Default|GetStarsEarned)))

(event EventBeginPlay
  (CallFunction|Init)
  (CallFunction|Set-Up))

(fn ConstructionScript)

(fn CalculateScore
  (params (ItemsBought :type Integer) (ItemsCarried :type Integer))
  (Variables|Default|SetPointsEarned (+ (* ItemsBought 2) (- ItemsCarried ItemsBought))))