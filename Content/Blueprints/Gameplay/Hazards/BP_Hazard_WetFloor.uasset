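; BP_Hazard_WetFloor is a wet floor hazard with a trigger box that the construction script sizes from XSize and YSize.
; Its begin and end overlap events only cast the other actor to ShopTillYaDropPawn, with no further effect.
; Disconnected logic holds the intended slip: a forward launch, zero friction and boosted speed, plus a restore of movement values with friction returning after a delay.
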(event OnComponentBeginOverlap(Box)
  (params (OverlappedComponent :type Primitive%20Component%20Object%20Reference) (OtherActor :type Actor%20Object%20Reference) (OtherComp :type Primitive%20Component%20Object%20Reference) (OtherBodyIndex :type Integer) (bFromSweep :type Boolean) (SweepResult :type Hit%20Result%20Structure%20%28by%20ref%29))
  (bind _asshop_till_ya_drop_pawn (Utilities|Casting|CastToShopTillYaDropPawn OtherActor)))

(event OnComponentEndOverlap(Box)
  (params (OverlappedComponent :type Primitive%20Component%20Object%20Reference) (OtherActor :type Actor%20Object%20Reference) (OtherComp :type Primitive%20Component%20Object%20Reference) (OtherBodyIndex :type Integer))
  (bind _asshop_till_ya_drop_pawn (Utilities|Casting|CastToShopTillYaDropPawn OtherActor)))

(fn ConstructionScript
  (Components|Box|SetBoxExtent (Variables|Default|GetBox) (Math|Vector|MakeVector (Variables|Default|GetXSize) (Variables|Default|GetYSize) 32.0) true))