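; AI controller that moves a BaseAI pawn back and forth along a spline path once StartMovement is called.
; A timeline, rate-scaled by spline length over max walk speed, feeds points along the spline to MoveToLocation.
; The controller's own actor-hit event flip-flops the timeline between reverse and forward.
; The random BP_Spline pick is disconnected, so this graph never sets SplinePathRef.
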(event Custom|RunFlipped
  (Components|Timeline|SetPlayRate (Variables|Default|GetMove) (/ 1.0 (Variables|Default|GetDuration)))
  (bind _alpha (Timeline|Move Reverse)
    (:Update
      (Variables|Default|SetAlpha _alpha)
      (AI|Navigation|MovetoLocation (Spline|GetLocationatDistanceAlongSpline (Variables|/Game/Blueprints/AI/BP_Spline.BP_Spline_C|GetSpline%20Path (Variables|Default|GetSplinePathRef)) (Math|Float|Lerp 0.0 (Spline|GetSplineLength (Variables|/Game/Blueprints/AI/BP_Spline.BP_Spline_C|GetSpline%20Path (Variables|Default|GetSplinePathRef))) (Variables|Default|GetAlpha)) "World") -1.0 true true false true 0))))

(event Custom|FlipMovement
  (Utilities|FlowControl|FlipFlop
    (:A
      (CallFunction|RunFlipped))
    (:B
      (CallFunction|RunNormal))))

(event Custom|RunNormal
  (Components|Timeline|SetPlayRate (Variables|Default|GetMove) (/ 1.0 (Variables|Default|GetDuration)))
  (bind _alpha (Timeline|Move Play)
    (:Update
      (Variables|Default|SetAlpha _alpha)
      (AI|Navigation|MovetoLocation (Spline|GetLocationatDistanceAlongSpline (Variables|/Game/Blueprints/AI/BP_Spline.BP_Spline_C|GetSpline%20Path (Variables|Default|GetSplinePathRef)) (Math|Float|Lerp 0.0 (Spline|GetSplineLength (Variables|/Game/Blueprints/AI/BP_Spline.BP_Spline_C|GetSpline%20Path (Variables|Default|GetSplinePathRef))) (Variables|Default|GetAlpha)) "World") -1.0 true true false true 0))))

(event Custom|StartMovement
  (EventDispatchers|BindEventtoActorHit (delegate Custom|FlipMovement))
  (Utilities|FlowControl|Sequence
    (:then_0
      (bind _asbase_ai (Utilities|Casting|CastToBaseAI (Pawn|GetControlledPawn)))
      (Variables|Default|SetAIPawn _asbase_ai)
      (Variables|Default|SetDuration (/ (Spline|GetSplineLength (Variables|/Game/Blueprints/AI/BP_Spline.BP_Spline_C|GetSpline%20Path (Variables|Default|GetSplinePathRef))) (Variables|/Script/Engine.CharacterMovementComponent|GetMaxWalkSpeed (Variables|/Script/Engine.Character|GetCharacterMovement _asbase_ai))))
      (Default|Start _asbase_ai))
    (:then_1
      (CallFunction|RunNormal))))

(fn ConstructionScript)