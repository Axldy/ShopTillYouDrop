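; BaseAI is an AI-controlled character that knocks back other characters touching its HitArea.
; On BeginPlay it applies its walk speed and caches its BasicAI_Controller.
; When a Character overlaps HitArea and that controller is valid, it calls the controller's ActorHit and launches the character along Arrow1's forward vector.
; A DoOnce reset after a one-second delay serves as the hit cooldown, while non-character overlaps reset it immediately.
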(event OnComponentBeginOverlap(HitArea)
  (params (OverlappedComponent :type Primitive%20Component%20Object%20Reference) (OtherActor :type Actor%20Object%20Reference) (OtherComp :type Primitive%20Component%20Object%20Reference) (OtherBodyIndex :type Integer) (bFromSweep :type Boolean) (SweepResult :type Hit%20Result%20Structure%20%28by%20ref%29))
  (bind _aicontroller (Variables|Default|GetAIController))
  (Utilities|FlowControl|DoOnce false :!label _label
    (:Completed
      (bind _ascharacter (Utilities|Casting|CastToCharacter OtherActor)
        (:then
          (Utilities|IsValid _aicontroller
            (:Is%20Valid
              (Default|CallActorHit _aicontroller)
              (Character|LaunchCharacter _ascharacter (* (Math|Vector|GetForwardVector (Variables|Default|GetArrow1)) 2e+03) false false))
            (:Is%20Not%20Valid
              _))
          (Utilities|FlowControl|Delay 1.0)
          (goto _label Reset))
        (:CastFailed
          (goto _label Reset))))))

(event EventBeginPlay
  (Variables|/Script/Engine.CharacterMovementComponent|SetMaxWalkSpeed (Variables|Character|GetCharacterMovement) (Variables|Default|GetWalk%20Speed))
  (bind _asbasic_ai_controller (Utilities|Casting|CastToBasicAI_Controller (Pawn|GetController)))
  (Variables|Default|SetAIController _asbasic_ai_controller))

(fn ConstructionScript)