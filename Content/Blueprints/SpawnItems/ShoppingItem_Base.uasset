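; Base shopping pickup for Shop Till Ya Drop that the player collects to gain weight and extra drop time.
; On init it moves randomly within a box, rolls a weight, takes its spawner's mesh and sets the pawn's target location.
; The location sent to the manager is a separate random roll from the actual position.
; Pawn overlap updates pawn stats, notifies the manager and destroys the item; overlap-avoidance logic is unwired.
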(event OnComponentBeginOverlap(Box)
  (params (OverlappedComponent :type Primitive%20Component%20Object%20Reference) (OtherActor :type Actor%20Object%20Reference) (OtherComp :type Primitive%20Component%20Object%20Reference) (OtherBodyIndex :type Integer) (bFromSweep :type Boolean) (SweepResult :type Hit%20Result%20Structure%20%28by%20ref%29))
  (bind _asshop_till_ya_drop_pawn (Utilities|Casting|CastToShopTillYaDropPawn OtherActor))
  (bind _result (Math|Integer|IncrementInt (Variables|/Game/Blueprints/Character/ShopTillYaDropPawn.ShopTillYaDropPawn_C|GetItemsPickedUp _asshop_till_ya_drop_pawn))
    (:%20%20
      (Variables|/Game/Blueprints/Character/ShopTillYaDropPawn.ShopTillYaDropPawn_C|SetItemsPickedUp _asshop_till_ya_drop_pawn _result)
      (Variables|/Game/Blueprints/Character/ShopTillYaDropPawn.ShopTillYaDropPawn_C|SetWeight _asshop_till_ya_drop_pawn (+ (Variables|/Game/Blueprints/Character/ShopTillYaDropPawn.ShopTillYaDropPawn_C|GetWeight _asshop_till_ya_drop_pawn) (Variables|Default|GetWeight)))
      (Variables|/Game/Blueprints/Character/ShopTillYaDropPawn.ShopTillYaDropPawn_C|SetTimeTillDrop _asshop_till_ya_drop_pawn (+ (Variables|/Game/Blueprints/Character/ShopTillYaDropPawn.ShopTillYaDropPawn_C|GetTimeTillDrop _asshop_till_ya_drop_pawn) 5.0))
      (Default|CallCheckWeight _asshop_till_ya_drop_pawn)
      (Default|CallCheckforItemPickUp (Variables|Default|GetManager))
      (Actor|DestroyActor))))

(event Custom|CheckLocationForOverlap)

(event Custom|SetLocation
  (bind _origin (Variables|Default|GetOrigin))
  (bind _boxextent (Variables|Default|GetBoxExtent))
  (bind _returnvalue (Math|Random|RandomPointinBoundingBox _origin _boxextent))
  (Variables|Default|SetItemLocation _returnvalue)
  (Transformation|SetActorLocation _returnvalue false false)
  (Default|GetCurrentLocation (Variables|Default|GetManager) (Variables|Default|GetItemLocation)))

(event Custom|Init
  (params (Spawner :type Item%20Spawner%20Object%20Reference) (Manager :type Game%20Manager%20Object%20Reference))
  (Variables|Default|SetSpawner Spawner)
  (Variables|Default|SetManager Manager)
  (CallFunction|SetUpItem))

(event Custom|SetUpItem
  (CallFunction|SetLocation)
  (Variables|Default|SetWeight (Math|Random|RandomFloatinRange 5.0 1e+01))
  (Components|StaticMesh|SetStaticMesh (Variables|Default|GetMesh) (Variables|/Game/Blueprints/GameControl/Spawn/ItemSpawner.ItemSpawner_C|GetItemToSpawn (Variables|Default|GetSpawner)))
  (bind _asshop_till_ya_drop_pawn (Utilities|Casting|CastToShopTillYaDropPawn (Game|GetPlayerCharacter 0)))
  (Variables|/Game/Blueprints/Character/ShopTillYaDropPawn.ShopTillYaDropPawn_C|SetTarget%20Location _asshop_till_ya_drop_pawn (Transformation|GetActorLocation)))

(event EventBeginPlay)

(fn ConstructionScript)