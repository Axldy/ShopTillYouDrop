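; Base pickup actor that adds five seconds to the overlapping ShopTillYaDropPawn's TimeTillDrop.
; Init stores its spawner and manager, moves the item to a random point within a bounding box and starts a timed despawn.
; Timelines scale the item up on BeginPlay and back down before it is destroyed.
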(event OnComponentBeginOverlap(Box)
  (params (OverlappedComponent :type Primitive%20Component%20Object%20Reference) (OtherActor :type Actor%20Object%20Reference) (OtherComp :type Primitive%20Component%20Object%20Reference) (OtherBodyIndex :type Integer) (bFromSweep :type Boolean) (SweepResult :type Hit%20Result%20Structure%20%28by%20ref%29))
  (bind _asshop_till_ya_drop_pawn (Utilities|Casting|CastToShopTillYaDropPawn OtherActor))
  (Variables|/Game/Blueprints/Character/ShopTillYaDropPawn.ShopTillYaDropPawn_C|SetTimeTillDrop _asshop_till_ya_drop_pawn (+ (Variables|/Game/Blueprints/Character/ShopTillYaDropPawn.ShopTillYaDropPawn_C|GetTimeTillDrop _asshop_till_ya_drop_pawn) 5.0))
  (Actor|DestroyActor))

(event Custom|Destroy%20Actor
  (bind _newtrack_0 (Timeline|Timeline_1 ReverseFromEnd)
    (:Update
      (Transformation|SetActorScale3D (Math|Vector|Lerp(Vector) "0, 0, 0" "1.000000,1.000000,1.000000" _newtrack_0)))
    (:Finished
      (Actor|DestroyActor))))

(event Custom|SetLocation
  (bind _origin (Variables|Default|GetOrigin))
  (bind _boxextent (Variables|Default|GetBoxExtent))
  (bind _returnvalue (Math|Random|RandomPointinBoundingBox _origin _boxextent))
  (Variables|Default|SetItemLocation _returnvalue)
  (Transformation|SetActorLocation _returnvalue false false))

(event Custom|Init
  (params (Spawner :type Objective%20Item%20Spawner%20Object%20Reference) (Manager :type Game%20Manager%20Object%20Reference))
  (Variables|Default|SetSpawner Spawner)
  (Variables|Default|SetManager Manager)
  (CallFunction|SetUpItem))

(event Custom|SetUpItem
  (CallFunction|SetLocation)
  (Utilities|Time|SetTimerbyEvent (delegate Custom|Destroy%20Actor) 2e+01))

(event EventBeginPlay
  (bind _newtrack_0 (Timeline|Timeline_0 Play)
    (:Update
      (Transformation|SetActorScale3D (Math|Vector|Lerp(Vector) "0, 0, 0" "1.000000,1.000000,1.000000" _newtrack_0)))))

(fn ConstructionScript)