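; Shelf item prop that randomizes the colors of its static mesh when play begins.
; BeginPlay makes four independent random picks from six color materials, one for each fixed group of material slots.
; Each group and color pair has its own SetTo function that hardcodes the slot indices, so the picks run as chained switches.
; The construction script is empty, so the random colors are applied only at runtime.
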(event EventBeginPlay
  (switch int (Math|Random|RandomIntegerinRange 0 5)
    (:0
      (|SetToWhite))
    (:1
      (|SetToRed))
    (:2
      (|SetToGreen))
    (:3
      (|SetToYellow))
    (:4
      (|SetToLightBrown))
    (:5
      (|SetToBlue)))
  (switch int (Math|Random|RandomIntegerinRange 0 5)
    (:0
      (|SetToWhite2))
    (:1
      (|SetToRed2))
    (:2
      (|SetToGreen2))
    (:3
      (|SetToYellow2))
    (:4
      (|SetToLightBrown2))
    (:5
      (|SetToBlue2)))
  (switch int (Math|Random|RandomIntegerinRange 0 5)
    (:0
      (|SetToWhite3))
    (:1
      (|SetToRed3))
    (:2
      (|SetToGreen3))
    (:3
      (|SetToYellow3))
    (:4
      (|SetToLightBrown3))
    (:5
      (|SetToBlue3)))
  (switch int (Math|Random|RandomIntegerinRange 0 5)
    (:0
      (|SetToWhite4))
    (:1
      (|SetToRed4))
    (:2
      (|SetToGreen4))
    (:3
      (|SetToYellow4))
    (:4
      (|SetToLightBrown4))
    (:5
      (|SetToBlue4))))

(fn ConstructionScript)