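; Shelf item prop that gives its static mesh a random solid color when play begins.
; BeginPlay rolls a random integer and calls one of six SetTo color functions.
; Each function applies a single color material to all eleven hard-coded material slots of the mesh.
; The construction script is empty, so the random color is only applied at runtime.
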(event EventBeginPlay
  (switch int (Math|Random|RandomIntegerinRange 0 5)
    (:0
      (|SetToWhite))
    (:1
      (|SetToRed))
    (:2
      (|SetToGreen))
    (:3
      (|SetToYellow))
    (:4
      (|SetToLightBrown))
    (:5
      (|SetToBlue))))

(fn ConstructionScript)